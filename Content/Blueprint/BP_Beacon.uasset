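; BP_Beacon is a capturable team beacon that can be unset, blue or red.
; On BeginPlay it snaps its mesh to the ground using a downward projectile path prediction.
; Capture calls S_Capture, which switches on current state and team to set BeaconState and remove the beacon from GM_GameMap's control arrays.
; The BeaconState RepNotify swaps light and mesh materials, registers team-owned beacons with the game mode and updates team control.
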(event Custom|S_HitGround
  (bind _staticmesh (Variables|Default|GetStaticMesh))
  ;[0.3113 0.2418 0.4427] Hit Ground
  (bind _outhit (Class|GameplayStatics|BlueprintPredictProjectilePathbyTraceChannel (Transformation|GetWorldLocation _staticmesh) "0, 0,-500.000000" true 0.0 "ECC_Visibility" false (Utilities|Array|MakeArray self) "None"))
  (if (.bblockinghit _outhit)
    (Transformation|SetWorldLocation _staticmesh (.impactpoint _outhit) false true)))

(event Custom|S_Capture
  (bind _self self)
  ;[0.397 0.603 1] Change color
  (switch Utilities|FlowControl|Switch|SwitchonEnum_Team (Variables|Default|GetBeaconState)
    (:NewEnumerator0
      (switch Utilities|FlowControl|Switch|SwitchonEnum_Team (stale EventCapture Team)
        (:NewEnumerator1
          (Variables|Default|SetBeaconState "NewEnumerator0" :!label _label)
          ;;[1 0.4023 0.1599] Remove from Old Array
          (bind _asgm_game_map (Utilities|Casting|CastToGM_GameMap (Game|GetGameMode) :!label _label_2))
          (Utilities|Array|RemoveItem (Variables|/Game/Levels/GameMap/GM_GameMap.GM_GameMap_C|GetRedControlArray _asgm_game_map) _self))
        (:NewEnumerator2
          (Variables|Default|SetBeaconState "NewEnumerator1" :!label _label_3)
          (bind _asgm_game_map_2 (Utilities|Casting|CastToGM_GameMap (Game|GetGameMode) :!label _label_4))
          (Utilities|Array|RemoveItem (Variables|/Game/Levels/GameMap/GM_GameMap.GM_GameMap_C|GetBlueControlArray _asgm_game_map_2) _self))))
    (:NewEnumerator1
      (switch Utilities|FlowControl|Switch|SwitchonEnum_Team (stale EventCapture Team)
        (:NewEnumerator0
          (Variables|Default|SetBeaconState "NewEnumerator2" :!label _label_5)
          (Utilities|FlowControl|Sequence
            (:then_0
              (goto _label_4))
            (:then_1
              (goto _label_2))))
        (:NewEnumerator2
          (goto _label_3))))
    (:NewEnumerator2
      (switch Utilities|FlowControl|Switch|SwitchonEnum_Team (stale EventCapture Team)
        (:NewEnumerator0
          (goto _label_5))
        (:NewEnumerator1
          (goto _label))))))

(event EventBeginPlay
  ;[0.3113 0.2418 0.4427] Hit Ground
  (CallFunction|SHitGround))

(event EventCapture
  (params (Team :type Enum_Team%20Enum :default "NewEnumerator0"))
  ;[0.397 0.603 1] Change color
  (CallFunction|SCapture))

(fn ConstructionScript)

(fn OnRepBeaconState
  (bind _self self)
  (bind _cone (Variables|Default|GetCone))
  (bind _staticmesh (Variables|Default|GetStaticMesh))
  ;[0.5688 0.1973 1] Change Material for match team owning
  (switch Utilities|FlowControl|Switch|SwitchonEnum_Team (Variables|Default|GetBeaconState)
    (:NewEnumerator0
      (Rendering|Material|SetMaterialbyName _cone "MI_LighthouseLight" "/Game/LightHouse/M_LighthouseLightNone.M_LighthouseLightNone")
      (Rendering|Material|SetMaterialbyName _staticmesh "Material_002" "/Game/LightHouse/M_BeaconWhite.M_BeaconWhite"))
    (:NewEnumerator1
      (Rendering|Material|SetMaterialbyName _cone "MI_LighthouseLight" "/Game/LightHouse/MI_LighthouseLightBlue.MI_LighthouseLightBlue")
      (Rendering|Material|SetMaterialbyName _staticmesh "Material_002" "/Game/LightHouse/M_BeaconBlue.M_BeaconBlue")
      ;[0.3656 0.688 1] Add in Control Array
      (bind _asgm_game_map (Utilities|Casting|CastToGM_GameMap (Game|GetGameMode)))
      (Utilities|Array|AddUnique (Variables|/Game/Levels/GameMap/GM_GameMap.GM_GameMap_C|GetBlueControlArray _asgm_game_map) _self)
      (bind _asgm_game_map_2 (Utilities|Casting|CastToGM_GameMap (Game|GetGameMode) :!label _label))
      (Default|SUpdateTeamControl _asgm_game_map_2))
    (:NewEnumerator2
      (Rendering|Material|SetMaterialbyName _cone "MI_LighthouseLight" "/Game/LightHouse/MI_LighthouseLightRed.MI_LighthouseLightRed")
      (Rendering|Material|SetMaterialbyName _staticmesh "Material_002" "/Game/LightHouse/M_BeaconRed.M_BeaconRed")
      (bind _asgm_game_map_3 (Utilities|Casting|CastToGM_GameMap (Game|GetGameMode)))
      (Utilities|Array|AddUnique (Variables|/Game/Levels/GameMap/GM_GameMap.GM_GameMap_C|GetRedControlArray _asgm_game_map_3) _self)
      (goto _label))))