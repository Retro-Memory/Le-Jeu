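; BP_Timer is a reusable timer Blueprint that counts down from, or up to, a given time in seconds.
; StartTimer initializes values behind a DoOnce and starts a looping timer event that steps ActualTime by the update frequency.
; PauseTimer pauses the handle, and AddTimeToTimer adjusts ActualTime according to direction to add time.
; Reaching the limit clears the handle and calls ResetTimer, which resets the DoOnce.
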(event Custom|StartTimer
  (params (IsCountDown? :type Boolean) (TimeIn%20S :type Float%20%28single-precision%29) (InitialDelayIn%20S :type Float%20%28single-precision%29) (UpdateFrequencyIn%20S :type Float%20%28single-precision%29))
  ;[0.2714 0.4115 0.2139] Timer set
  (Utilities|FlowControl|Sequence
    (:then_0
      (Utilities|FlowControl|DoOnce false
        (:Completed
          (bind _output_get (Variables|Timer|SetTimeIn%20S TimeIn%20S))
          (Variables|Timer|SetUpdate%20Frequency%20in%20S UpdateFrequencyIn%20S)
          (Variables|Timer|SetIsCountDown? IsCountDown?)
          (if IsCountDown?
            (Variables|Timer|SetActualTime _output_get)
            (else
              (Variables|Timer|SetActualTime 0.0))))))
    (:then_1
      ;[1 0.2782 0.8195] Clock
      (bind _returnvalue (Utilities|Time|SetTimerbyEvent (delegate Custom|Timer) UpdateFrequencyIn%20S true InitialDelayIn%20S))
      (Variables|Timer|SetTimerRef _returnvalue))))

(event Custom|Timer
  ;[0.2118 1 0.4018] Timer update
  (if (Variables|Timer|GetIsCountDown?)
    (bind _output_get (Variables|Timer|SetActualTime (- (Variables|Timer|GetActualTime) (Variables|Timer|GetUpdate%20Frequency%20in%20S))))
    (if (<= _output_get 0.0)
      (Utilities|Time|ClearandInvalidateTimerbyHandle (Variables|Timer|GetTimerRef))
      ;[0.724 0.06033 0.06033] Call Reset
      (CallFunction|ResetTimer :!label _label))
    (else
      (bind _output_get_2 (Variables|Timer|SetActualTime (+ (Variables|Timer|GetActualTime) (Variables|Timer|GetUpdate%20Frequency%20in%20S))))
      (if (>= _output_get_2 (Variables|Timer|GetTimeIn%20S))
        (Utilities|Time|ClearandInvalidateTimerbyHandle (Variables|Timer|GetTimerRef))
        (goto _label)))))

(event Custom|PauseTimer
  ;[0.7778 0.1739 1] Pause Clock
  (Utilities|Time|PauseTimerbyHandle (Variables|Timer|GetTimerRef)))

(event Custom|AddTimeToTimer
  (params (TimeToAddIn%20S :type Float%20%28single-precision%29))
  ;[0.2077 0.6715 1] Add or Substract Time
  (if (Variables|Timer|GetIsCountDown?)
    (Variables|Timer|SetActualTime (+ (Variables|Timer|GetActualTime) TimeToAddIn%20S))
    (else
      (Variables|Timer|SetActualTime (- (Variables|Timer|GetActualTime) TimeToAddIn%20S)))))

(event Custom|ResetTimer
  ;[1 0 0] Reset Timer
  ;[0.2714 0.4115 0.2139] Timer set
  (Utilities|FlowControl|DoOnce false) ; enters at Reset
)

(fn ConstructionScript)