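; Beacon system actor that spawns a square, flat grid of BP_Beacon actors centered on its scene component.
; The BuildGrid event derives even spacing from GridSize and RowsColumns, then offsets a starting corner in negative X and Y.
; Nested loops step along X for rows and Y for columns, spawning a scaled-up beacon at each point.
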(event Custom|BuildGrid
  (bind _rows_columns (Variables|Default|GetRows&Columns))
  (bind _scene (Variables|Default|GetScene))
  (bind _returnvalue (Transformation|GetWorldLocation _scene))
  ;[0.2357 0.7777 1] Getting Grid size and Offsets
  (Variables|Default|SetOffset%20X/Y (/ (* (Variables|Default|GetGridSize) 100) _rows_columns))
  ;[1 0.1446 0.1248] Rows
  (Variables|Default|SetTopCorner (Math|Vector|MakeVector (- (.x _returnvalue) (* (Math|Conversions|ToFloat(Integer) (Variables|Default|GetOffset%20X/Y)) (/ (Math|Conversions|ToFloat(Integer) (+ (Variables|Default|GetRows&Columns) 2)) 2.0))) (- (.y _returnvalue) (* (Math|Conversions|ToFloat(Integer) (Variables|Default|GetOffset%20X/Y)) (/ (Math|Conversions|ToFloat(Integer) (+ (Variables|Default|GetRows&Columns) 2)) 2.0))) (.z _returnvalue)))
  (for _index (range 0 _rows_columns)
    (bind _output_get (Variables|Default|SetTopCorner (+ (Variables|Default|GetTopCorner) (Math|Vector|MakeVector (Math|Conversions|ToFloat(Integer) (Variables|Default|GetOffset%20X/Y)) 0.0 0.0))))
    ;[0.5113 1 0.2222] Columns
    (Variables|Default|SetColumns _output_get)
    (for _index_2 (range 0 _rows_columns)
      (bind _output_get_2 (Variables|Default|SetColumns (+ (Variables|Default|GetColumns) (Math|Vector|MakeVector 0.0 (Math|Conversions|ToFloat(Integer) (Variables|Default|GetOffset%20X/Y)) 0.0))))
      ;[0.5481 0.2557 1] Spawn Beacon
      (Game|SpawnActorfromClass "/Game/Blueprint/Beacons/BP_Beacon.BP_Beacon_C" (Math|Transform|MakeTransform _output_get_2 "0, 0, 0" "3.000000,3.000000,3.000000") "Undefined" 0 0))))

(fn ConstructionScript)