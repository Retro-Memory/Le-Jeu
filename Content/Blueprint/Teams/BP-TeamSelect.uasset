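; BP-TeamSelect is a lobby trigger that assigns a player to the blue or red team when their character overlaps its box.
; The construction script applies a configurable material to the border, and the overlap checks whether that material is M_BlueBorder to choose the team.
; It swaps team tags on the PlayerController, updates the character's team, then reports the player as ready to GM_Lobby.
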(event OnComponentBeginOverlap(Box)
  (params (OverlappedComponent :type Primitive%20Component%20Object%20Reference) (OtherActor :type Actor%20Object%20Reference) (OtherComp :type Primitive%20Component%20Object%20Reference) (OtherBodyIndex :type Integer) (bFromSweep :type Boolean) (SweepResult :type Hit%20Result%20Structure%20%28by%20ref%29))
  ;[0.3395 1 0.5822] Attach Tag to Controller
  (bind _asch_character (Utilities|Casting|CastToCh_Character OtherActor))
  (bind _asplayer_controller (Utilities|Casting|CastToPlayerController (Game|GetInstigatorController _asch_character)))
  (if (== (Rendering|Material|GetMaterial (Variables|Default|GetBorder) 0) "/Game/Assets/Spawn/Materials/M_BlueBorder.M_BlueBorder")
    (Utilities|Array|AddUnique (Variables|/Script/Engine.Actor|GetTags _asplayer_controller) "BlueTeam")
    (Utilities|Array|RemoveItem (Variables|/Script/Engine.Actor|GetTags _asplayer_controller) "RedTeam")
    (else
      (Utilities|Array|AddUnique (Variables|/Script/Engine.Actor|GetTags _asplayer_controller) "RedTeam")
      (Utilities|Array|RemoveItem (Variables|/Script/Engine.Actor|GetTags _asplayer_controller) "BlueTeam")))
  (Default|UpdateTeam _asch_character)
  (bind _asgm_lobby (Utilities|Casting|CastToGM_Lobby (Game|GetGameMode)))
  (Default|PlayerReady _asgm_lobby _asch_character))

(fn ConstructionScript
  (Rendering|Material|SetMaterial (Variables|Default|GetBorder) 0 (Variables|Default|GetMaterial)))