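; Weapon actor that configures itself at BeginPlay from the DataT_Weapons row matching its WeaponName enum.
; It stores the row as WeaponStats, then creates a skeletal mesh with the row's skin and transform, ignoring all collision channels.
; It also spawns a deactivated Niagara muzzle flash, with color, boost, delay, power and width fed through SetNiagaraParameter.
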(event EventBeginPlay
  ;[0.3327 1 0] Apply Data to Weapon's Stat
  (bind _returnvalue (Utilities|GetDataTableRow "/Game/Blueprint/Weapons/DataT_Weapons.DataT_Weapons" (Utilities|String|StringToName (Utilities|String|EnumtoString (Variables|Default|GetWeaponName))))
    (:then
      (bind _output_get (Variables|Default|SetWeaponStats _returnvalue))
      (bind _returnvalue_2 (AddComponent|AddSkeletalMeshComponent false (.WeaponTransform (Utilities|Struct|BreakStruct_WeaponStats _output_get))))
      (Class|SkinnedMeshComponent|SetSkeletalMesh _returnvalue_2 (.WeaponSkin (Utilities|Struct|BreakStruct_WeaponStats _output_get)) true)
      (bind _returnvalue_3 (AddComponent|AddNiagaraComponent false (.Transform (Utilities|Struct|BreakStruct_MuzzleFlash_Parameter (.Muzzle_Flash (Utilities|Struct|BreakStruct_WeaponStats _output_get))))))
      (bind _output_get_2 (Variables|Default|SetMuzzle_flash _returnvalue_3))
      (Class|NiagaraComponent|SetAsset _output_get_2 (.NiagaraSystem (Utilities|Struct|BreakStruct_MuzzleFlash_Parameter (.Muzzle_Flash (Utilities|Struct|BreakStruct_WeaponStats _output_get)))) true)
      (Components|Activation|Deactivate _returnvalue_3)
      (CallFunction|SetNiagaraParameter _returnvalue_3 (.Color (Utilities|Struct|BreakStruct_MuzzleFlash_Parameter (.Muzzle_Flash (Utilities|Struct|BreakStruct_WeaponStats _output_get)))) (.Color_Boost (Utilities|Struct|BreakStruct_MuzzleFlash_Parameter (.Muzzle_Flash (Utilities|Struct|BreakStruct_WeaponStats _output_get)))) (.Delay (Utilities|Struct|BreakStruct_MuzzleFlash_Parameter (.Muzzle_Flash (Utilities|Struct|BreakStruct_WeaponStats _output_get)))) (.Power (Utilities|Struct|BreakStruct_MuzzleFlash_Parameter (.Muzzle_Flash (Utilities|Struct|BreakStruct_WeaponStats _output_get)))) (.Width (Utilities|Struct|BreakStruct_MuzzleFlash_Parameter (.Muzzle_Flash (Utilities|Struct|BreakStruct_WeaponStats _output_get)))))
      (Collision|SetCollisionResponsetoAllChannels _returnvalue_2 "ECR_Ignore"))))

(fn ConstructionScript)

(fn SetNiagaraParameter
  (params (Muzzle :type Niagara%20Component%20Object%20Reference) (Color :type Linear%20Color%20Structure) (Color_Boost :type Float%20%28single-precision%29) (Delay :type Float%20%28single-precision%29) (Power :type Float%20%28single-precision%29) (Width :type Float%20%28single-precision%29))
  ;[0 0.591 1] Set Parameters of the Muzzle Flash
  (Effects|Components|ParticleSystem|SetColorParameter Muzzle "Color" Color)
  (Effects|Components|ParticleSystem|SetFloatParameter Muzzle "Color_Boost" Color_Boost)
  (Effects|Components|ParticleSystem|SetFloatParameter Muzzle "Delay" Delay)
  (Effects|Components|ParticleSystem|SetFloatParameter Muzzle "Power" Power)
  (Effects|Components|ParticleSystem|SetFloatParameter Muzzle "Width" Width))