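; Game Mode for the game map, running team beacon-control scoring and player spawning for Blue and Red.
; A looping timer, started once, adds each team's weighted beacon count to the current round's score and pushes it to GSt_GameMap.
; After a retriggerable join delay, it checks session capacity, kicks extras and spawns characters at PlayerStarts named by number and team tag.
; Controller tags carry across level swaps, and respawns use random team starts after a delay.
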(event Custom|S_StartCountPoint
  ;[0.02077 0.000322 0.02083] Start Timer for point
  (bind _returnvalue (Utilities|Time|SetTimerbyEvent (delegate Custom|S_IncreasePoint) (Variables|Score|GetScoreUpdateFrequency) true 0.1))
  (Variables|Score|SetTimerStartCountPoint_Ref _returnvalue))

(event Custom|S_IncreasePoint
  (bind _round (Variables|Game|GetRound))
  (bind _round_2 (Variables|Game|GetRound))
  ;[0.3021 0 0.249] Updating score by Team and Round
  (Utilities|FlowControl|Sequence
    (:then_0
      ;;[0.1582 0.8296 1] Getting length of Array, which is equal to the number of beacons ows by each team
      (Variables|Score|SetBlueControl (* (Utilities|Array|Length (Variables|ControlByTeam|GetBlueControlArray)) (Variables|ControlbyTeam|GetFactorControlBlue)))
      (Variables|Score|SetRedControl (* (Utilities|Array|Length (Variables|ControlbyTeam|GetRedControlArray)) (Variables|ControlbyTeam|GetFactorControlRed))))
    (:then_1
      (if (== _round_2 1)
        (bind _structout (Utilities|Struct|SetmembersinStruct_PointScorebyTeam (Variables|Score|GetScoring) (+ (.Score_R1_Tblue (Utilities|Struct|BreakStruct_PointScorebyTeam (Variables|Score|GetScoring))) (Variables|Score|GetBlueControl)) (+ (.Score_R1_TRed (Utilities|Struct|BreakStruct_PointScorebyTeam (Variables|Score|GetScoring))) (Variables|Score|GetRedControl))))
        (bind _asgst_game_map (Utilities|Casting|CastToGSt_GameMap (Game|GetGameState)))
        (bind _output_get (Variables|/Game/Levels/GameMap/GSt_GameMap.GSt_GameMap_C|SetScoring _asgst_game_map _structout))
        (bind _output_get_2 (Variables|/Game/Levels/GameMap/GSt_GameMap.GSt_GameMap_C|SetBlueControl _asgst_game_map (Variables|Score|GetBlueControl)))
        (bind _output_get_3 (Variables|/Game/Levels/GameMap/GSt_GameMap.GSt_GameMap_C|SetRedControl _asgst_game_map (Variables|Score|GetRedControl)))
        (Default|CallUpdateScore _asgst_game_map _output_get _round _output_get_2 _output_get_3)
        (elif (== _round_2 2)
          (bind _structout_2 (Utilities|Struct|SetmembersinStruct_PointScorebyTeam (Variables|Score|GetScoring) (+ (.Score_R2_Tblue (Utilities|Struct|BreakStruct_PointScorebyTeam (Variables|Score|GetScoring))) (Variables|Score|GetBlueControl)) (+ (.Score_R2_Tred (Utilities|Struct|BreakStruct_PointScorebyTeam (Variables|Score|GetScoring))) (Variables|Score|GetRedControl))))
          (bind _asgst_game_map_2 (Utilities|Casting|CastToGSt_GameMap (Game|GetGameState)))
          (bind _output_get_4 (Variables|/Game/Levels/GameMap/GSt_GameMap.GSt_GameMap_C|SetScoring _asgst_game_map_2 _structout_2))
          (bind _output_get_5 (Variables|/Game/Levels/GameMap/GSt_GameMap.GSt_GameMap_C|SetBlueControl _asgst_game_map_2 (Variables|Score|GetBlueControl)))
          (bind _output_get_6 (Variables|/Game/Levels/GameMap/GSt_GameMap.GSt_GameMap_C|SetRedControl _asgst_game_map_2 (Variables|Score|GetRedControl)))
          (Default|CallUpdateScore _asgst_game_map_2 _output_get_4 _round _output_get_5 _output_get_6)
          (else
            (bind _structout_3 (Utilities|Struct|SetmembersinStruct_PointScorebyTeam (Variables|Score|GetScoring) (+ (.Score_R3_Tblue (Utilities|Struct|BreakStruct_PointScorebyTeam (Variables|Score|GetScoring))) (Variables|Score|GetBlueControl)) (+ (.Score_R3_Tred (Utilities|Struct|BreakStruct_PointScorebyTeam (Variables|Score|GetScoring))) (Variables|Score|GetRedControl))))
            (bind _asgst_game_map_3 (Utilities|Casting|CastToGSt_GameMap (Game|GetGameState)))
            (bind _output_get_7 (Variables|/Game/Levels/GameMap/GSt_GameMap.GSt_GameMap_C|SetScoring _asgst_game_map_3 _structout_3))
            (bind _output_get_8 (Variables|/Game/Levels/GameMap/GSt_GameMap.GSt_GameMap_C|SetBlueControl _asgst_game_map_3 (Variables|Score|GetBlueControl)))
            (bind _output_get_9 (Variables|/Game/Levels/GameMap/GSt_GameMap.GSt_GameMap_C|SetRedControl _asgst_game_map_3 (Variables|Score|GetRedControl)))
            (Default|CallUpdateScore _asgst_game_map_3 _output_get_7 _round _output_get_8 _output_get_9)))))))

(event Custom|S_UpdateTeamControl
  ;[0.5946 1 0.3488] Update Control of each Team
  ;;[0.01896 0.09938 0.1198] Launch Timer Once by Round
  (Utilities|FlowControl|DoOnce false
    (:Completed
      (CallFunction|SStartCountPoint))))

(event Custom|S_Respawn
  (params (InputPin :type Controller%20Object%20Reference))
  ;[0.5103 1 0.9901] Wait For Respawn
  (Utilities|FlowControl|Delay (Variables|Game|GetTimeToRespawn))
  (bind _returnvalue (Game|SpawnActorfromClass "/Game/Character/Ch_Character.Ch_Character_C" (Transformation|GetActorTransform (Class|GameModeBase|FindPlayerStart InputPin (Utilities|String|ToString(Text) (Utilities|Text|FormatText "{Number}{Team}" (Math|Random|RandomIntegerinRange 0 9) (Utilities|Array|Get(acopy) (Variables|/Script/Engine.Actor|GetTags InputPin)))))) "Undefined" 0 0))
  (Pawn|Possess InputPin _returnvalue))

(event EventOnLogout
  (params (ExitingController :type Controller%20Object%20Reference))
  ;[1 0.3177 0.3177 0.272] Remove Player Controller Ref on Logout
  (bind _asplayer_controller (Utilities|Casting|CastToPlayerController ExitingController))
  (Utilities|Array|RemoveItem (Variables|Game|GetPlayers%20Controllers) _asplayer_controller))

(event EventOnSwapPlayerControllers
  (params (OldPC :type Player%20Controller%20Object%20Reference) (NewPC :type Player%20Controller%20Object%20Reference))
  ;[0 0 0] Transit Tags between Levels
  (Variables|/Script/Engine.Actor|SetTags NewPC (Variables|/Script/Engine.Actor|GetTags OldPC)))

(event EventHandleStartingNewPlayer
  (params (NewPlayer :type Player%20Controller%20Object%20Reference))
  (bind _returnvalue (Game|GetGameState))
  (bind _playerarray (Variables|/Script/Engine.GameStateBase|GetPlayerArray _returnvalue))
  (bind _returnvalue_2 (Utilities|Array|Length _playerarray))
  ;[0.7542 0.3488 1] Testing if enough players to start
  (Utilities|Array|AddUnique (Variables|Game|GetPlayers%20Controllers) NewPlayer)
  (Utilities|FlowControl|RetriggerableDelay 1.0)
  (bind (_numconnections _numprivateconnections _bislan _bisdedicated _ballowinvites _ballowjoininprogress _bisanticheatenabled _builduniqueid _extrasettings) (Class|AdvancedSessionsLibrary|GetSessionSettings)
    (:OnSuccess
      (if (< _numconnections _returnvalue_2)
        (bind (_arrayindex _arrayelement) (Utilities|Array|ReverseforEachLoop (Variables|Game|GetPlayers%20Controllers))
          (:LoopBody
            (if (> _arrayindex _numconnections)
              (Class|AdvancedSessionsLibrary|KickPlayer _arrayelement "Too many Player, we are sorry...")))
          (:Completed
            (|UpdateSession _extrasettings _numconnections 0 false false false true false :!label _label
              (:OnSuccess
                (for (_array_element _array_index) (Variables|Game|GetPlayers%20Controllers)
                  (bind _returnvalue_3 (Game|SpawnActorfromClass "/Game/Character/Ch_Character.Ch_Character_C" (Transformation|GetActorTransform (Class|GameModeBase|FindPlayerStart _array_element (Utilities|String|ToString(Text) (Utilities|Text|FormatText "{Number}{Team}" _array_index (Utilities|Array|Get(acopy) (Variables|/Script/Engine.Actor|GetTags _array_element)))))) "Undefined" 0 0))
                  (Pawn|Possess _array_element _returnvalue_3))))))
        (elif (== _numconnections _returnvalue_2)
          (goto _label))))))

(fn ConstructionScript)