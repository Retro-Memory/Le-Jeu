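; Lobby GameMode that manages joining players and launches the team match.
; After a debounced delay on login, it checks session capacity and kicks surplus controllers from its tracked list.
; Ready players are sorted into Red or Blue by controller tag; equal teams filling the session trigger a session update and delayed server travel to GameMap.
; Controller tags are copied on controller swap so they carry between levels.
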(event Custom|PlayerReady
  (params (PlayerCharacter :type Ch%20Character%20Object%20Reference))
  (bind _redteamplayers (Variables|Default|GetRedTeamPlayers))
  (bind _blueteamplayers (Variables|Default|GetBlueTeamPlayers))
  (bind _returnvalue (Utilities|Array|Length _blueteamplayers))
  ;[0.08731 0.2097 1] Start if enough Player and equal Teams members
  (bind _asplayer_controller (Utilities|Casting|CastToPlayerController (Pawn|GetController PlayerCharacter)))
  (if (Actor|ActorHasTag _asplayer_controller "RedTeam")
    (Utilities|Array|AddUnique _redteamplayers PlayerCharacter)
    (Utilities|Array|RemoveItem _blueteamplayers PlayerCharacter)
    (if (== (Utilities|Array|Length _redteamplayers) _returnvalue) :!label _label
      (if (== (* _returnvalue 2) (Variables|Default|GetNum%20Connections))
        (bind (_numconnections _numprivateconnections _bislan _bisdedicated _ballowinvites _ballowjoininprogress _bisanticheatenabled _builduniqueid _extrasettings) (Class|AdvancedSessionsLibrary|GetSessionSettings)
          (:OnSuccess
            (|UpdateSession _extrasettings _numconnections _numprivateconnections _bislan _bisdedicated _ballowinvites _ballowjoininprogress _bisanticheatenabled
              (:OnSuccess
                (Utilities|FlowControl|Delay 3.0)
                (Development|ExecuteConsoleCommand "serverTravel GameMap" 0)))))))
    (elif (Actor|ActorHasTag _asplayer_controller "BlueTeam")
      (Utilities|Array|AddUnique _blueteamplayers PlayerCharacter)
      (Utilities|Array|RemoveItem _redteamplayers PlayerCharacter)
      (goto _label))))

(event EventOnLogout
  (params (ExitingController :type Controller%20Object%20Reference))
  ;[1 0.3177 0.3177 0.272] Remove Player Controller Ref on Logout
  (bind _asplayer_controller (Utilities|Casting|CastToPlayerController ExitingController))
  (Utilities|Array|RemoveItem (Variables|Default|GetPlayersControllers) _asplayer_controller))

(event EventOnSwapPlayerControllers
  (params (OldPC :type Player%20Controller%20Object%20Reference) (NewPC :type Player%20Controller%20Object%20Reference))
  ;[0 0 0] Transit Tags between Levels
  (Variables|/Script/Engine.Actor|SetTags NewPC (Variables|/Script/Engine.Actor|GetTags OldPC)))

(event EventPostLogin
  (params (NewPlayer :type Player%20Controller%20Object%20Reference))
  ;[0.7542 0.3488 1] Kicking if too much Player
  (Utilities|Array|AddUnique (Variables|Default|GetPlayersControllers) NewPlayer)
  (Utilities|FlowControl|RetriggerableDelay 1.0)
  (bind _numconnections (Class|AdvancedSessionsLibrary|GetSessionSettings)
    (:OnSuccess
      (Variables|Default|SetNum%20Connections _numconnections)
      (if (< _numconnections (Utilities|Array|Length (Variables|/Script/Engine.GameStateBase|GetPlayerArray (Game|GetGameState))))
        (bind (_arrayindex _arrayelement) (Utilities|Array|ReverseforEachLoop (Variables|Default|GetPlayersControllers))
          (:LoopBody
            (if (> _arrayindex _numconnections)
              (Class|AdvancedSessionsLibrary|KickPlayer _arrayelement "Too many Player, we are sorry..."))))))))

(fn ConstructionScript)